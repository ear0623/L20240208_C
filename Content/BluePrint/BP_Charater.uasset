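; Character Blueprint that moves the character from the MoveFoward and MoveRight input axes.
; Each axis adds movement input along the forward or right vector of the full control rotation, scaled by the axis value.
; The axes also set the IsForwad and IsRight flags while non-zero and clear them at zero.
; BeginPlay, overlap, Tick and the construction script are empty.
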(event EventBeginPlay)

(event Collision|EventActorBeginOverlap
  (params (OtherActor :type Actor%20Object%20Reference)))

(event EventTick
  (params (DeltaSeconds :type Float%20%28single-precision%29)))

(event Input|AxisEvents|InputAxisMoveFoward
  (params (AxisValue :type Float%20%28single-precision%29))
  (bind _returnvalue (Pawn|GetControlRotation :!class /Script/Engine.Pawn))
  (bind _returnvalue_2 (Math|Vector|GetForwardVector _returnvalue))
  (if (!= AxisValue 0.0)
    (Variables|Default|SetbIsForwad true)
    (Pawn|Input|AddMovementInput _returnvalue_2 AxisValue false)
    (else
      (Variables|Default|SetbIsForwad false)
      (Pawn|Input|AddMovementInput _returnvalue_2 AxisValue false))))

(event Input|AxisEvents|InputAxisMoveRight
  (params (AxisValue :type Float%20%28single-precision%29))
  (if (!= AxisValue 0.0)
    (Variables|Default|SetbIsRight true)
    (Pawn|Input|AddMovementInput (Math|Vector|GetRightVector (Pawn|GetControlRotation :!class /Script/Engine.Pawn)) AxisValue false)
    (else
      (Variables|Default|SetbIsRight false))))

(fn ConstructionScript)